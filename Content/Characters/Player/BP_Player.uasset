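; BP_Player is the player character, with Enhanced Input movement, look, sprinting and single-weapon pickup and drop.
; Movement follows control rotation, and sprint swaps the max walk speed between walking and running values.
; PickupBox tracks an overlapped BP_AR4; pickup copies its WeaponData, destroys it and shows the mesh on WeaponHolster.
; Drop clears the holster and spawns a BP_AR4 carrying that data in front of the player.
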(event OnComponentBeginOverlap(PickupBox)
  (params (OverlappedComponent :type Primitive%20Component%20Object%20Reference) (OtherActor :type Actor%20Object%20Reference) (OtherComp :type Primitive%20Component%20Object%20Reference) (OtherBodyIndex :type Integer) (bFromSweep :type Boolean) (SweepResult :type Hit%20Result%20Structure%20%28by%20ref%29))
  (bind _asbp_ar4 (Utilities|Casting|CastToBP_AR4 OtherActor))
  (Variables|Default|SetDetectWeapon _asbp_ar4))

(event OnComponentEndOverlap(PickupBox)
  (params (OverlappedComponent :type Primitive%20Component%20Object%20Reference) (OtherActor :type Actor%20Object%20Reference) (OtherComp :type Primitive%20Component%20Object%20Reference) (OtherBodyIndex :type Integer))
  (Variables|Default|SetDetectWeapon 0))

(event Input|EnhancedActionEvents|EnhancedInputActionIA_Pickup
  (params (ActionValue :type Boolean) (ElapsedSeconds :type Float%20%28double-precision%29) (TriggeredSeconds :type Float%20%28double-precision%29) (InputAction :type Input%20Action%20Object%20Reference :default "/Game/Input/IA_Pickup.IA_Pickup"))
  (:Started
    (Utilities|IsValid (Variables|Default|GetDetectWeapon)
      (:Is%20Valid
        (Variables|Default|SetWeapon (Variables|/Game/Weapons/BP_AR4.BP_AR4_C|GetWeaponData (Variables|Default|GetDetectWeapon)))
        (Actor|DestroyActor (Variables|Default|GetDetectWeapon))
        (Variables|Default|SetDetectWeapon 0)
        (Components|SkeletalMesh|SetSkeletalMeshAsset (Variables|Default|GetWeaponHolster) (Variables|/Game/Weapons/Data/BP_WeaponData.BP_WeaponData_C|GetMesh (Variables|Default|GetWeapon)))))))

(event Input|EnhancedActionEvents|EnhancedInputActionIA_Drop
  (params (ActionValue :type Boolean) (ElapsedSeconds :type Float%20%28double-precision%29) (TriggeredSeconds :type Float%20%28double-precision%29) (InputAction :type Input%20Action%20Object%20Reference :default "/Game/Input/IA_Drop.IA_Drop"))
  (:Started
    (Utilities|IsValid (Variables|Default|GetWeapon)
      (:Is%20Valid
        (Components|SkeletalMesh|SetSkeletalMeshAsset (Variables|Default|GetWeaponHolster) 0)
        (Game|SpawnActorfromClass "/Game/Weapons/BP_AR4.BP_AR4_C" (Math|Transform|MakeTransform (+ (Transformation|GetActorLocation) (* (Math|Vector|GetForwardVector (Pawn|GetControlRotation :!class /Script/Engine.Pawn)) (Variables|Default|GetDropWeapon_Offset))) "0, 0, 0" "1.000000,1.000000,1.000000") "Undefined" "MultiplyWithRoot" 0 (Variables|Default|GetWeapon) 0)
        (Variables|Default|SetWeapon 0)))))

(event Input|EnhancedActionEvents|EnhancedInputActionIA_Look
  (params (ActionValue :type Vector%202D%20Structure) (ElapsedSeconds :type Float%20%28double-precision%29) (TriggeredSeconds :type Float%20%28double-precision%29) (InputAction :type Input%20Action%20Object%20Reference :default "/Game/Input/IA_Look.IA_Look"))
  (Pawn|Input|AddControllerYawInput (.x ActionValue))
  (Pawn|Input|AddControllerPitchInput (.y ActionValue)))

(event Input|EnhancedActionEvents|EnhancedInputActionIA_Move
  (params (ActionValue :type Vector%202D%20Structure) (ElapsedSeconds :type Float%20%28double-precision%29) (TriggeredSeconds :type Float%20%28double-precision%29) (InputAction :type Input%20Action%20Object%20Reference :default "/Game/ThirdPerson/Input/Actions/IA_Move.IA_Move"))
  (bind _returnvalue (Pawn|GetControlRotation :!class /Script/Engine.Pawn))
  (Pawn|Input|AddMovementInput (Math|Vector|GetRightVector (Pawn|GetControlRotation :!class /Script/Engine.Pawn)) (.x ActionValue) false)
  (Pawn|Input|AddMovementInput (Math|Vector|GetForwardVector (Math|Rotator|MakeRotator (.roll _returnvalue) 0.0 (.yaw _returnvalue))) (.y ActionValue) false))

(event Input|EnhancedActionEvents|EnhancedInputActionIA_Sprint
  (params (ActionValue :type Boolean) (ElapsedSeconds :type Float%20%28double-precision%29) (TriggeredSeconds :type Float%20%28double-precision%29) (InputAction :type Input%20Action%20Object%20Reference :default "/Game/Input/IA_Sprint.IA_Sprint"))
  (bind _charactermovement (Variables|Character|GetCharacterMovement))
  (:Started
    (Variables|/Script/Engine.CharacterMovementComponent|SetMaxWalkSpeed _charactermovement (Variables|Default|GetRunningVelocity)))
  (:Completed
    (Variables|/Script/Engine.CharacterMovementComponent|SetMaxWalkSpeed _charactermovement (Variables|Default|GetWalkingVelocity))))

(event EventBeginPlay
  (bind _asplayer_controller (Utilities|Casting|CastToPlayerController (Pawn|GetController)))
  (Input|AddMappingContext (PlayerController|LocalPlayerSubsystems|GetEnhancedInputLocalPlayerSubsystem _asplayer_controller) "/Game/Input/IMC_Player.IMC_Player" 0 "(bIgnoreAllPressedKeysUntilRelease=True,bForceImmediately=False,bNotifyUserSettings=False)")
  (Variables|/Script/Engine.CharacterMovementComponent|SetMaxWalkSpeed (Variables|Character|GetCharacterMovement) (Variables|Default|GetWalkingVelocity)))

(fn ConstructionScript)